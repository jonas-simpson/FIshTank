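; BP_Bubble is a physics-driven bubble actor that splits into smaller bubbles when it hits something.
; Root bubbles pick a random size and horizontal velocity on spawn, while children take the size and velocity set by their parent.
; On hit, a bubble above the smallest size spawns two children one size down, pushed apart perpendicular to the hit normal plus its current velocity.
; Every bubble destroys itself on hit.
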(event `self.ReceiveBeginPlay`
  (bind _spherecol (`self.SphereCol`))
  (bind _startspeedmax (`self.StartSpeedMax`))
  (bind _returnvalue (`KismetMathLibrary.Conv_IntToDouble` (`self.Size`)))
  (bind _returnvalue_2 (* (`self.StartSpeedMax`) -1.0))
  (bind _returnvalue_3 (`KismetMathLibrary.MakeVector` _returnvalue _returnvalue _returnvalue))
  (`KismetSystemLibrary.Delay` 0.01)
  (if (`self.IsChild`)
    (`SceneComponent.SetWorldScale3D` _spherecol _returnvalue_3)
    (`PrimitiveComponent.AddImpulse` _spherecol (`self.InitialVelocity`) "None" true)
    (else
      (set `self.Size` (`KismetMathLibrary.RandomIntegerInRange` 1 3))
      (`SceneComponent.SetWorldScale3D` _spherecol _returnvalue_3)
      (bind _output_get (set `self.InitialVelocity` (`KismetMathLibrary.MakeVector` (`KismetMathLibrary.RandomFloatInRange` _returnvalue_2 _startspeedmax) (`KismetMathLibrary.RandomFloatInRange` _returnvalue_2 _startspeedmax))))
      (`PrimitiveComponent.SetPhysicsLinearVelocity` _spherecol _output_get false "None"))))

(event `self.SphereCol.OnComponentHit`
  (params (HitComponent :type "PrimitiveComponent Object Reference") (OtherActor :type "Actor Object Reference") (OtherComp :type "PrimitiveComponent Object Reference") (NormalImpulse :type "Vector Structure") (Hit :type "HitResult Structure (by ref)"))
  (bind _spherecol (`self.SphereCol`))
  (bind _returnvalue (`SceneComponent.K2_GetComponentToWorld` _spherecol))
  (bind _returnvalue_2 (* (`KismetMathLibrary.Cross_VectorVector` (`KismetMathLibrary.Normal` NormalImpulse) (`KismetMathLibrary.Vector_Up`)) (`self.CollisionMultiply`)))
  (if (> (`self.Size`) 1)
    (bind _returnvalue_3 (`PrimitiveComponent.GetPhysicsLinearVelocity` _spherecol "None"))
    (bind _returnvalue_4 (`|SpawnActorFromClass` "BP_Bubble_C" _returnvalue "AlwaysSpawn" "OverrideRootScale" null null))
    (set `/Game/Blueprints/BP_Bubble.IsChild` true _returnvalue_4)
    (set `/Game/Blueprints/BP_Bubble.InitialVelocity` (+ _returnvalue_2 _returnvalue_3) _returnvalue_4)
    (set `/Game/Blueprints/BP_Bubble.Size` (- (`self.Size`) 1) _returnvalue_4)
    (bind _returnvalue_5 (`|SpawnActorFromClass` "BP_Bubble_C" _returnvalue "AlwaysSpawn" "OverrideRootScale" null null))
    (set `/Game/Blueprints/BP_Bubble.IsChild` true _returnvalue_5)
    (set `/Game/Blueprints/BP_Bubble.InitialVelocity` (+ (* _returnvalue_2 -1.0) _returnvalue_3) _returnvalue_5)
    (set `/Game/Blueprints/BP_Bubble.Size` (- (`self.Size`) 1) _returnvalue_5))
  (`self.K2_DestroyActor`))

(fn `UserConstructionScript`)