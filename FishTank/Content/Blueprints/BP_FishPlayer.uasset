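; BP_FishPlayer is a player fish pawn with an unfinished movement prototype.
; The InputRotation axis applies a constant-falloff radial force to the collision component at RotSpeed strength, ignoring the axis value.
; ButtonForward toggles AcceleratePressed, but nothing in this graph reads it and Tick is empty.
; Controller yaw and forward movement input nodes are left disconnected, so they never run.
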(event `self.ReceiveTick`
  (params (DeltaSeconds :type "Float (single-precision)")))

(event `InputAxis|InputRotation`
  (params (AxisValue :type "Float (single-precision)"))
  ;[1 1 1] Movement - Rotate
  (`PrimitiveComponent.AddRadialForce` (`self.CollisionComponent`) (0.0 0.0 0.0) 0.0 (`self.RotSpeed`) "RIF_Constant" false))

(event `InputAction|ButtonForward`
  (params (Key :type "Key Structure"))
  (:`Pressed`
    (set `self.AcceleratePressed` true))
  (:`Released`
    (set `self.AcceleratePressed` false)))

(fn `UserConstructionScript`)