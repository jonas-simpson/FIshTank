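; Game mode Blueprint for a bubble game that tracks score and lives and spawns waves of BP_Bubble actors.
; SpawnBubbles runs at BeginPlay, increments the spawn count each call and scatters bubbles randomly within a flat box around the origin.
; CountBubbles starts another, larger wave when no bubbles remain.
; AddScore accumulates points, while SubtractLife restores lives and clears the score when the last life is lost.
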(event `self.ReceiveBeginPlay`
  ;[0 0.01154 1] BeginPlay - Spawn Bubbles
  (`self.SpawnBubbles`))

(event `AddScore`
  (params (ScoreToAdd :type Integer))
  ;[1 1 1] Add Score
  (set `self.TotalScore` (+ ScoreToAdd (`self.TotalScore`))))

(event `SubtractLife`
  (bind _totallives (`self.TotalLives`))
  ;[1 1 1] Subtract Lives / Reset Score
  (if (> _totallives 1)
    (set `self.TotalLives` (- _totallives 1))
    (else
      (set `self.TotalLives` 3)
      (set `self.TotalScore` 0))))

(event `CountBubbles`
  (bind _outactors (`GameplayStatics.GetAllActorsOfClass` "/Game/Blueprints/BP_Bubble.BP_Bubble_C"))
  (bind _output_get (set `self.NumBubbles` (`KismetArrayLibrary.Array_Length` _outactors)))
  (if (<= _output_get 0)
    (`self.SpawnBubbles`)))

(fn `SpawnBubbles`
  (bind _result (`/Engine/EditorBlueprintResources/StandardMacros.IncrementInt` (`self.NumBubblesToSpawn`))
    (:`  `
      (for _ (range (+ _result 1))
        (`|SpawnActorFromClass` "/Game/Blueprints/BP_Bubble.BP_Bubble_C" (`KismetMathLibrary.Conv_VectorToTransform` (`KismetMathLibrary.RandomPointInBoundingBox` (0.0 0.0 0.0) (1700.0 1000.0 0.0))) "AdjustIfPossibleButAlwaysSpawn" "OverrideRootScale" null null)))))

(fn `UserConstructionScript`)