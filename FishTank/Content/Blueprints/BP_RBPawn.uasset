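; BP_RBPawn is a player-controlled rigid-body pawn, moved entirely through physics on its SphereCol component.
; The InputForward axis applies a mass-independent force along the sphere's forward vector, scaled by MoveAccel.
; Turn actions add a yaw angular impulse of RotSpeed as a velocity change on press and the opposite impulse on release, so turning needs no per-frame update.
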(event `InputAction|TurnClockwise`
  (params (Key :type "Key Structure"))
  (bind _spherecol (`self.SphereCol`))
  (bind _returnvalue (`KismetMathLibrary.MakeVector` 0.0 0.0 (`self.RotSpeed`)))
  ;[1 1 1] Movement - Rotate with Angular Impulse
  (:`Pressed`
    (`PrimitiveComponent.AddAngularImpulseInDegrees` _spherecol _returnvalue "None" true :!label _label))
  (:`Released`
    (`PrimitiveComponent.AddAngularImpulseInDegrees` _spherecol (* _returnvalue -1.0) "None" true :!label _label_2)))

(event `InputAction|TurnCounterClockwise`
  (params (Key :type "Key Structure"))
  ;[1 1 1] Movement - Rotate with Angular Impulse
  (:`Pressed`
    (goto _label_2))
  (:`Released`
    (goto _label)))

(event `InputAxis|InputForward`
  (params (AxisValue :type "Float (single-precision)"))
  ;[1 1 1] Movement - Accelerate Forward with Linear Force
  (`PrimitiveComponent.AddForce` (`self.SphereCol`) (* (`SceneComponent.GetForwardVector` (`self.SphereCol`)) (* AxisValue (`self.MoveAccel`))) "None" true))

(fn `UserConstructionScript`)